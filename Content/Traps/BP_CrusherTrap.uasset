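; BP_CrusherTrap is a looping crusher trap that kills the first-person character on contact.
; Two timelines, ResetPos and Crush, drive the Cube's relative Z in alternation, starting with ResetPos on BeginPlay.
; A random pause precedes each crush and a fixed pause precedes each reset.
; Overlapping the Box applies huge damage to BP_FirstPersonCharacter only, regardless of the crusher's current phase.
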(event OnComponentBeginOverlap(Box)
  (params (OverlappedComponent :type Primitive%20Component%20Object%20Reference) (OtherActor :type Actor%20Object%20Reference) (OtherComp :type Primitive%20Component%20Object%20Reference) (OtherBodyIndex :type Integer) (bFromSweep :type Boolean) (SweepResult :type Hit%20Result%20Structure%20%28by%20ref%29))
  (bind _asbp_first_person_character (Utilities|Casting|CastToBP_FirstPersonCharacter OtherActor))
  (Game|Damage|ApplyDamage _asbp_first_person_character 676942.0 0 0 "/Script/Engine.DamageType"))

(event EventBeginPlay
  (bind _cube (Variables|Default|GetCube))
  (bind _relativelocation (Variables|/Script/Engine.SceneComponent|GetRelativeLocation _cube))
  (bind _relativelocation_2 (Variables|/Script/Engine.SceneComponent|GetRelativeLocation _cube))
  (bind _newtrack_0 (Timeline|ResetPos Play)
    (:Update
      (Transformation|SetRelativeLocation _cube (Math|Vector|MakeVector (.x _relativelocation_2) (.y _relativelocation_2) (* _newtrack_0 1e+03)) false false))
    (:Finished
      (Utilities|FlowControl|Delay (Math|Random|RandomFloatinRange 2.0 5.0))
      (bind _newtrack_0_2 (Timeline|Crush PlayFromStart)
        (:Update
          (Transformation|SetRelativeLocation _cube (Math|Vector|MakeVector (.x _relativelocation) (.y _relativelocation) (* _newtrack_0_2 1e+02)) false false))
        (:Finished
          (Utilities|FlowControl|Delay 2.0)
          (Timeline|ResetPos PlayFromStart))))))

(fn ConstructionScript)