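; BP_SawBlade is a trap actor with a moving saw that deals lethal-scale damage to the first-person character on touching its KillBox.
; On BeginPlay it takes a random yaw, then runs the SawTween timeline, which alternates between forward and reverse playback using a Reverse flag.
; Each timeline update adds the scaled track value to the model's current relative X, so movement accumulates rather than following an absolute position.
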(event OnComponentBeginOverlap(KillBox)
  (params (OverlappedComponent :type Primitive%20Component%20Object%20Reference) (OtherActor :type Actor%20Object%20Reference) (OtherComp :type Primitive%20Component%20Object%20Reference) (OtherBodyIndex :type Integer) (bFromSweep :type Boolean) (SweepResult :type Hit%20Result%20Structure%20%28by%20ref%29))
  (bind _asbp_first_person_character (Utilities|Casting|CastToBP_FirstPersonCharacter OtherActor))
  (Game|Damage|ApplyDamage _asbp_first_person_character 235465.0 0 0))

(event EventBeginPlay
  (bind _replacewithmodel (Variables|Default|GetReplaceWithModel))
  (bind _relativelocation (Variables|/Script/Engine.SceneComponent|GetRelativeLocation _replacewithmodel))
  (Transformation|SetActorRotation (Math|Rotator|MakeRotator 0.0 0.0 (Math|Random|RandomFloatinRange 0.0 359.0)))
  (bind _newtrack_0 (Timeline|SawTween Play)
    (:Update
      (Transformation|SetRelativeLocation (Variables|Default|GetReplaceWithModel) (Math|Vector|MakeVector (+ (* _newtrack_0 2e+01) (.x _relativelocation)) (.y _relativelocation) (.z _relativelocation)) false false))
    (:Finished
      (if (Variables|Default|Getreverse)
        (Variables|Default|Setreverse false)
        (Timeline|SawTween Reverse)
        (else
          (Variables|Default|Setreverse true)
          (Timeline|SawTween PlayFromStart))))))

(fn ConstructionScript)