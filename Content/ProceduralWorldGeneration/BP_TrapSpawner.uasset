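; BP_TrapSpawner is a procedural world generation actor that randomly places a trap within an area.
; On BeginPlay, or when its Spawn event is called, it rolls a four-in-five chance to spawn.
; It picks a random class from its Traps array and spawns it at a random point inside the TrapSpawnSomewhereHere box, adjusting for collisions but always spawning.
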(event Custom|Spawn
  (bind _trapspawnsomewherehere (Variables|Default|GetTrapSpawnSomewhereHere))
  (bind _traps (Variables|Default|GetTraps))
  (if (not (== (Math|Random|RandomIntegerinRange 0 4) 0))
    (Game|SpawnActorfromClass (Utilities|Array|Get(acopy) _traps (Math|Random|RandomInteger (Utilities|Array|Length _traps))) (Math|Transform|MakeTransform (Math|Random|RandomPointinBoundingBox (Transformation|GetWorldLocation _trapspawnsomewherehere) (Variables|/Script/Engine.BoxComponent|GetBoxExtent _trapspawnsomewherehere)) "0, 0, 0" "1.000000,1.000000,1.000000") "AdjustIfPossibleButAlwaysSpawn" "MultiplyWithRoot" 0 0)))

(event EventBeginPlay
  (bind _trapspawnsomewherehere (Variables|Default|GetTrapSpawnSomewhereHere))
  (bind _traps (Variables|Default|GetTraps))
  (if (not (== (Math|Random|RandomIntegerinRange 0 4) 0))
    (Game|SpawnActorfromClass (Utilities|Array|Get(acopy) _traps (Math|Random|RandomInteger (Utilities|Array|Length _traps))) (Math|Transform|MakeTransform (Math|Random|RandomPointinBoundingBox (Transformation|GetWorldLocation _trapspawnsomewherehere) (Variables|/Script/Engine.BoxComponent|GetBoxExtent _trapspawnsomewherehere)) "0, 0, 0" "1.000000,1.000000,1.000000") "AdjustIfPossibleButAlwaysSpawn" "MultiplyWithRoot" 0 0)))

(fn ConstructionScript)