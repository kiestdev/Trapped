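; BP_Soda is a consumable pickup that gives the first-person character a temporary walk speed boost.
; Overlapping its LookatBox shows an interaction prompt, and IA_Interact attaches the soda to the character as the equipped item, destroying the box.
; Consume runs once, detaching the soda, raising walk speed, then restoring it after a delay and destroying itself.
; End overlap hides the prompt but never clears LookedAt.
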(event OnComponentBeginOverlap(LookatBox)
  (params (OverlappedComponent :type Primitive%20Component%20Object%20Reference) (OtherActor :type Actor%20Object%20Reference) (OtherComp :type Primitive%20Component%20Object%20Reference) (OtherBodyIndex :type Integer) (bFromSweep :type Boolean) (SweepResult :type Hit%20Result%20Structure%20%28by%20ref%29))
  (bind _outactors (Actor|GetAllActorsOfClass "/Game/FirstPerson/Blueprints/BP_FirstPersonCharacter.BP_FirstPersonCharacter_C"))
  (bind _array_element (Utilities|Array|ForEachLoopwithBreak _outactors :!label _label)
    (:LoopBody
      (if (== _array_element OtherActor)
        (Variables|Default|SetLookedAt true)
        (Variables|Default|SetPlayerLookingAt _array_element)
        (goto _label Break)))
    (:Completed
      (Default|DisplayInteractivePrompt (Variables|Default|GetPlayerLookingAt) true (Variables|Default|GetPromptText)))))

(event OnComponentEndOverlap(LookatBox)
  (params (OverlappedComponent :type Primitive%20Component%20Object%20Reference) (OtherActor :type Actor%20Object%20Reference) (OtherComp :type Primitive%20Component%20Object%20Reference) (OtherBodyIndex :type Integer))
  (bind _outactors (Actor|GetAllActorsOfClass "/Game/FirstPerson/Blueprints/BP_FirstPersonCharacter.BP_FirstPersonCharacter_C"))
  (bind _array_element (Utilities|Array|ForEachLoopwithBreak _outactors :!label _label)
    (:LoopBody
      (if (== _array_element 0)
        (Variables|Default|SetLookedAt true)
        (Variables|Default|SetPlayerLookingAt _array_element)
        (goto _label Break)))
    (:Completed
      (Default|DisplayInteractivePrompt (Variables|Default|GetPlayerLookingAt) false (Variables|Default|GetPromptText)))))

(event Custom|Consume
  (bind _playerlookingat (Variables|Default|GetPlayerLookingAt))
  (bind _charactermovement (Variables|/Script/Engine.Character|GetCharacterMovement _playerlookingat))
  (if (not (Variables|Default|GetBeingUsed))
    (Variables|Default|SetBeingUsed true)
    (Variables|/Script/Engine.CharacterMovementComponent|SetMaxWalkSpeed _charactermovement (* (Variables|/Script/Engine.CharacterMovementComponent|GetMaxWalkSpeed _charactermovement) 1.25))
    (Development|PrintString "Hello")
    (Transformation|DetachFromActor "KeepRelative" "KeepRelative" "KeepRelative")
    (Utilities|FlowControl|Delay 1e+01)
    (Variables|/Script/Engine.CharacterMovementComponent|SetMaxWalkSpeed _charactermovement (/ (Variables|/Script/Engine.CharacterMovementComponent|GetMaxWalkSpeed _charactermovement) 1.25))
    (Actor|DestroyActor)))

(event Input|EnhancedActionEvents|EnhancedInputActionIA_Interact
  (params (ActionValue :type Boolean) (ElapsedSeconds :type Float%20%28double-precision%29) (TriggeredSeconds :type Float%20%28double-precision%29) (InputAction :type Input%20Action%20Object%20Reference :default "/Game/Input/Actions/IA_Interact.IA_Interact"))
  (if (Variables|Default|GetLookedAt)
    (Transformation|AttachComponentToComponent (Variables|/Game/FirstPerson/Blueprints/BP_FirstPersonCharacter.BP_FirstPersonCharacter_C|Getsodagoeshere (Variables|Default|GetPlayerLookingAt)) "None" "SnapToTarget" "SnapToTarget" "KeepRelative" true)
    (Components|DestroyComponent (Variables|Default|GetLookatBox))
    (Variables|/Game/FirstPerson/Blueprints/BP_FirstPersonCharacter.BP_FirstPersonCharacter_C|SetCurrentItemEquipped (Variables|Default|GetPlayerLookingAt) self)))

(fn ConstructionScript)