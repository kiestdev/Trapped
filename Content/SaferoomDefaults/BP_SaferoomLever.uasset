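; BP_SaferoomLever is an interactable lever that opens a saferoom door and closes it when the player passes an exit trigger.
; A look-at overlap box toggles the player's interaction prompt and gates the Interact input.
; The first valid press, guarded by DoOnce, stores the door's Z and plays a timeline that raises it.
; Overlapping ExitBox reverses that timeline; map regeneration is noted as planned but not implemented.
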(event OnComponentBeginOverlap(LookatBox)
  (params (OverlappedComponent :type Primitive%20Component%20Object%20Reference) (OtherActor :type Actor%20Object%20Reference) (OtherComp :type Primitive%20Component%20Object%20Reference) (OtherBodyIndex :type Integer) (bFromSweep :type Boolean) (SweepResult :type Hit%20Result%20Structure%20%28by%20ref%29))
  (bind _asbp_first_person_character (Utilities|Casting|CastToBP_FirstPersonCharacter OtherActor))
  (Default|DisplayInteractivePrompt _asbp_first_person_character (Variables|Default|GetPromptText) true)
  (Variables|Default|SetLookedAt true)
  (Variables|Default|SetPlayerLookingAt _asbp_first_person_character))

(event OnComponentEndOverlap(LookatBox)
  (params (OverlappedComponent :type Primitive%20Component%20Object%20Reference) (OtherActor :type Actor%20Object%20Reference) (OtherComp :type Primitive%20Component%20Object%20Reference) (OtherBodyIndex :type Integer))
  (bind _asbp_first_person_character (Utilities|Casting|CastToBP_FirstPersonCharacter OtherActor))
  (Default|DisplayInteractivePrompt _asbp_first_person_character (Variables|Default|GetPromptText) false)
  (Variables|Default|SetLookedAt false)
  (Variables|Default|SetPlayerLookingAt 0))

(event OnComponentBeginOverlap(ExitBox)
  (params (OverlappedComponent :type Primitive%20Component%20Object%20Reference) (OtherActor :type Actor%20Object%20Reference) (OtherComp :type Primitive%20Component%20Object%20Reference) (OtherBodyIndex :type Integer) (bFromSweep :type Boolean) (SweepResult :type Hit%20Result%20Structure%20%28by%20ref%29))
  (bind _saferoomdoor (Variables|Default|GetSaferoomDoor))
  (bind _returnvalue (Transformation|GetActorTransform _saferoomdoor))
  (Utilities|Casting|CastToBP_FirstPersonCharacter OtherActor)
  ;[0.15 0.15 0.15 0.5] This will eventually cause the entire map to regenerate and stuff
  (bind _newtrack_0 (Timeline|SaferoomDoorOpen Reverse)
    (:Update
      (Transformation|SetActorTransform _saferoomdoor (Math|Transform|MakeTransform (Math|Vector|MakeVector (.x (.location _returnvalue)) (.y (.location _returnvalue)) (+ (* _newtrack_0 6e+02) (Variables|Default|GetActorLocation))) (.rotation _returnvalue) (.scale _returnvalue))))))

(event Input|EnhancedActionEvents|EnhancedInputActionIA_Interact
  (params (ActionValue :type Boolean) (ElapsedSeconds :type Float%20%28double-precision%29) (TriggeredSeconds :type Float%20%28double-precision%29) (InputAction :type Input%20Action%20Object%20Reference :default "/Game/Input/Actions/IA_Interact.IA_Interact"))
  (bind _saferoomdoor (Variables|Default|GetSaferoomDoor))
  (bind _returnvalue (Transformation|GetActorTransform _saferoomdoor))
  ;[0.15 0.15 0.15 0.5] This will eventually cause the entire map to regenerate and stuff
  (:Started
    (if (Variables|Default|GetLookedAt)
      (Utilities|FlowControl|DoOnce false
        (:Completed
          (Variables|Default|SetActorLocation (.z (.location _returnvalue)))
          (bind _newtrack_0 (Timeline|SaferoomDoorOpen Play)
            (:Update
              (Transformation|SetActorTransform _saferoomdoor (Math|Transform|MakeTransform (Math|Vector|MakeVector (.x (.location _returnvalue)) (.y (.location _returnvalue)) (+ (* _newtrack_0 6e+02) (Variables|Default|GetActorLocation))) (.rotation _returnvalue) (.scale _returnvalue))))))))))

(fn ConstructionScript)